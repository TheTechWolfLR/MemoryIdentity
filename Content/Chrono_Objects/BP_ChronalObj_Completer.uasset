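; Chronal puzzle object that the player moves along a spline to activate an interactable and, unless flagged as multi, start an NPC dialogue.
; A mission-change binding enables the trigger box only during the relevant mission parts.
; Player overlap highlights the cylinder and runs a timeline tied to Oroboros watch time that positions it along the spline.
; Leaving early resets the watch time and reverses the timeline, while finishing locks the route.
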(event `self.ReceiveBeginPlay`
  ; Set Collision During mission parts
  (bind _asbp_game_instance (cast `/Game/Chrono_MissionBPs/BP_GameInstance` (`GameplayStatics.GetGameInstance`)))
  (`PrimitiveComponent.SetCollisionEnabled` (`self.Box`) "QueryOnly")
  (add `/Game/Chrono_MissionBPs/BP_GameInstance.MissionWorldSetter` _asbp_game_instance (delegate `HandleStageChange`)))

(event `HandleStageChange`
  (params (`Mission Titel` :type Name) (`Mission Part` :type Name))
  ; Set Collision During mission parts
  (if (and (== `Mission Titel` (`self.RelevantMission`)) (`KismetArrayLibrary.Array_Contains` (`self.VisibleDuringParts`) `Mission Part`))
    (`PrimitiveComponent.SetCollisionEnabled` (`self.Box`) "QueryAndPhysics")
    (else
      (`PrimitiveComponent.SetCollisionEnabled` (`self.Box`) "NoCollision"))))

(event `self.Box.OnComponentBeginOverlap`
  (params (OverlappedComponent :type "PrimitiveComponent Object Reference") (OtherActor :type "Actor Object Reference") (OtherComp :type "PrimitiveComponent Object Reference") (OtherBodyIndex :type Integer) (bFromSweep :type Boolean) (SweepResult :type "HitResult Structure (by ref)"))
  (if (`self.ActorHasTag` OtherActor "Player")
    (if (not (`self.FinishedRoute`))
      (bind _asbp_third_person_character (cast `/Game/ThirdPerson/Blueprints/BP_ThirdPersonCharacter` OtherActor))
      (set `self.IsInsideArea` true)
      (`PrimitiveComponent.SetMaterial` (`self.Cylinder`) 0 "/Game/Chrono_Objects/Materials/M_ActiveChronalObject.M_ActiveChronalObject")
      (set `self.CharacterRef` _asbp_third_person_character)
      (bind (_direction _movebackward) (`Timeline|Timeline 1` :`NewTime` (* (`KismetMathLibrary.Conv_IntToDouble` (`/Game/ThirdPerson/Blueprints/BP_ThirdPersonCharacter.OroborosWatchTime` (`self.CharacterRef`))) (select `bool` (`self.IsMovingBackwards`) :`false` 0.01 :`true` -0.01)) :!label _label)
        (:`Update`
          (bind _returnvalue (* _movebackward (`SplineComponent.GetSplineLength` (`self.Spline`))))
          (`SceneComponent.K2_SetWorldLocationAndRotation` (`self.Cylinder`) (`SplineComponent.GetLocationAtDistanceAlongSpline` (`self.Spline`) _returnvalue "World") (`KismetMathLibrary.MakeRotator` (.roll (`SplineComponent.GetRotationAtDistanceAlongSpline` (`self.Spline`) _returnvalue "World")) (.pitch (`SplineComponent.GetRotationAtDistanceAlongSpline` (`self.Spline`) _returnvalue "World")) (.yaw (`SplineComponent.GetRotationAtDistanceAlongSpline` (`self.Spline`) _returnvalue "World"))) false false))
        (:`Finished`
          (set `self.FinishedRoute` true)
          (`PrimitiveComponent.SetMaterial` (`self.Cylinder`) 0 "/Game/Chrono_Objects/Materials/M_BaseChronalObject.M_BaseChronalObject")
          ; Set a bool on the interactor on, call the start dialog
          (set `/Game/Chrono_MissionBPs/BP_InteractableObject.Active?` true (`self.BP_InteractableObject`))
          (if (not (`self.IsThisMulti?`))
            (message `/Game/Chrono_Objects/BPI_DialogueCaller.CallDialogue` (`self.GetComponentByClass` (`self.NPCreffrence`) "/Game/DialogueShenanagins/BP_DialogueComponent.BP_DialogueComponent_C") (`self.GoToDialogueRow`))))))))

(event `self.Box.OnComponentEndOverlap`
  (params (OverlappedComponent :type "PrimitiveComponent Object Reference") (OtherActor :type "Actor Object Reference") (OtherComp :type "PrimitiveComponent Object Reference") (OtherBodyIndex :type Integer))
  (if (`self.ActorHasTag` OtherActor "Player")
    (if (not (`self.FinishedRoute`))
      (set `self.IsInsideArea` false)
      (`PrimitiveComponent.SetMaterial` (`self.Cylinder`) 0 "/Game/Chrono_Objects/Materials/M_BaseChronalObject.M_BaseChronalObject")
      (set `/Game/ThirdPerson/Blueprints/BP_ThirdPersonCharacter.OroborosWatchTime` 0 (`self.CharacterRef`))
      (goto _label :!via `Reverse`))))

(event `self.ReceiveTick`
  (params (DeltaSeconds :type "Float (single-precision)"))
  (if (`self.FinishedRoute`)
    _
    (elif (`self.IsInsideArea`)
      (goto _label :!via `SetNewTime`))))

(fn `UserConstructionScript`)