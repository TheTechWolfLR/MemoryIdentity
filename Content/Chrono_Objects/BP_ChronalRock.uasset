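; BP_ChronalRock is a rock whose sphere moves along a spline under the influence of the player's Oroboros watch.
; While the character is inside the trigger sphere, Tick sets the timeline's time, which is fed by the watch time scaled and signed by movement direction.
; The timeline output maps to distance along the spline.
; Leaving the trigger resets the character's watch time and reverses the timeline.
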(event `self.Sphere1.OnComponentBeginOverlap`
  (params (OverlappedComponent :type "PrimitiveComponent Object Reference") (OtherActor :type "Actor Object Reference") (OtherComp :type "PrimitiveComponent Object Reference") (OtherBodyIndex :type Integer) (bFromSweep :type Boolean) (SweepResult :type "HitResult Structure (by ref)"))
  (bind _asbp_third_person_character (cast `/Game/ThirdPerson/Blueprints/BP_ThirdPersonCharacter` OtherActor))
  (set `self.IsInsideArea` true)
  (set `self.CharacterRef` _asbp_third_person_character)
  (bind (_direction _movebackward) (`Timeline|Timeline` :`NewTime` (* (`KismetMathLibrary.Conv_IntToDouble` (`/Game/ThirdPerson/Blueprints/BP_ThirdPersonCharacter.OroborosWatchTime` (`self.CharacterRef`))) (select `bool` (`self.IsMovingBackwards`) :`false` 0.01 :`true` -0.01)) :!label _label)
    (:`Update`
      (`SceneComponent.K2_SetWorldLocation` (`self.Sphere`) (`SplineComponent.GetLocationAtDistanceAlongSpline` (`self.Spline`) (* _movebackward (`SplineComponent.GetSplineLength` (`self.Spline`))) "World") false false))))

(event `self.Sphere1.OnComponentEndOverlap`
  (params (OverlappedComponent :type "PrimitiveComponent Object Reference") (OtherActor :type "Actor Object Reference") (OtherComp :type "PrimitiveComponent Object Reference") (OtherBodyIndex :type Integer))
  (set `self.IsInsideArea` false)
  (set `/Game/ThirdPerson/Blueprints/BP_ThirdPersonCharacter.OroborosWatchTime` 0 (`self.CharacterRef`))
  (goto _label :!via `Reverse`))

(event `self.ReceiveTick`
  (params (DeltaSeconds :type "Float (single-precision)"))
  (if (`self.IsInsideArea`)
    (goto _label :!via `SetNewTime`)))

(fn `UserConstructionScript`)