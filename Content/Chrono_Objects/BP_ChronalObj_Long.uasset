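; BP_ChronalObj_Long is a chronal object whose cylinder moves along a spline, tied to the player's Ouroboros watch time.
; Entering the box swaps in an active material and plays a timeline that positions and rotates the cylinder along the spline.
; Leaving restores the material, zeroes watch time and reverses the timeline.
; Mission stage events reset watch time and show the actor only during relevant mission parts.
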(event `self.ReceiveBeginPlay`
  (bind _asbp_game_instance (cast `/Game/Chrono_MissionBPs/BP_GameInstance` (`GameplayStatics.GetGameInstance`)))
  (`self.SetActorHiddenInGame` true)
  (add `/Game/Chrono_MissionBPs/BP_GameInstance.MissionWorldSetter` _asbp_game_instance (delegate `HandleStageChange`)))

(event `self.Box.OnComponentBeginOverlap`
  (params (OverlappedComponent :type "PrimitiveComponent Object Reference") (OtherActor :type "Actor Object Reference") (OtherComp :type "PrimitiveComponent Object Reference") (OtherBodyIndex :type Integer) (bFromSweep :type Boolean) (SweepResult :type "HitResult Structure (by ref)"))
  (bind _asbp_third_person_character (cast `/Game/ThirdPerson/Blueprints/BP_ThirdPersonCharacter` OtherActor))
  (set `self.IsInsideArea` true)
  (`PrimitiveComponent.SetMaterial` (`self.Cylinder`) 0 "/Game/Chrono_Objects/Materials/M_ActiveChronalObject.M_ActiveChronalObject")
  (set `self.CharacterRef` _asbp_third_person_character)
  (bind (_direction _movebackward) (`Timeline|Timeline 1` :`NewTime` (* (`KismetMathLibrary.Conv_IntToDouble` (`/Game/ThirdPerson/Blueprints/BP_ThirdPersonCharacter.OroborosWatchTime` (`self.CharacterRef`))) (select `bool` (`self.IsMovingBackwards`) :`false` 0.01 :`true` -0.01)) :!label _label)
    (:`Update`
      (bind _returnvalue (* _movebackward (`SplineComponent.GetSplineLength` (`self.Spline`))))
      (`SceneComponent.K2_SetWorldLocationAndRotation` (`self.Cylinder`) (`SplineComponent.GetLocationAtDistanceAlongSpline` (`self.Spline`) _returnvalue "World") (`KismetMathLibrary.MakeRotator` (.roll (`SplineComponent.GetRotationAtDistanceAlongSpline` (`self.Spline`) _returnvalue "World")) (+ 90.0 (.pitch (`SplineComponent.GetRotationAtDistanceAlongSpline` (`self.Spline`) _returnvalue "World"))) (.yaw (`SplineComponent.GetRotationAtDistanceAlongSpline` (`self.Spline`) _returnvalue "World"))) false false))))

(event `HandleStageChange`
  (params (`Mission Titel` :type Name) (`Mission Part` :type Name))
  (set `/Game/ThirdPerson/Blueprints/BP_ThirdPersonCharacter.OroborosWatchTime` 0 (`self.CharacterRef`))
  (if (and (== `Mission Titel` (`self.RelevantMission`)) (`KismetArrayLibrary.Array_Contains` (`self.VisibleDuringParts`) `Mission Part`))
    (`self.SetActorHiddenInGame` false)
    (else
      (`self.SetActorHiddenInGame` true))))

(event `self.Box.OnComponentEndOverlap`
  (params (OverlappedComponent :type "PrimitiveComponent Object Reference") (OtherActor :type "Actor Object Reference") (OtherComp :type "PrimitiveComponent Object Reference") (OtherBodyIndex :type Integer))
  (set `self.IsInsideArea` false)
  (`PrimitiveComponent.SetMaterial` (`self.Cylinder`) 0 "/Game/Chrono_Objects/Materials/M_BaseChronalObject.M_BaseChronalObject")
  (set `/Game/ThirdPerson/Blueprints/BP_ThirdPersonCharacter.OroborosWatchTime` 0 (`self.CharacterRef`))
  (goto _label :!via `Reverse`))

(event `self.ReceiveTick`
  (params (DeltaSeconds :type "Float (single-precision)"))
  (if (`self.IsInsideArea`)
    (goto _label :!via `SetNewTime`)))

(fn `UserConstructionScript`)