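; Cinematic chronal object, an effigy actor that is positioned along the spline of a referenced SplinePath.
; MoveEffigy scales an alpha by the spline length and snaps the actor to the world location and rotation at that distance.
; The PositionState RepNotify prints the value and passes it through SetPositionState to MoveEffigy, so replicated changes drive the movement.
; An older Cylinder-based move with a pitch offset remains in the graph but never runs.
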(event `MoveEffigy`
  (params (`Set Move Alpha` :type "Float (double-precision)"))
  (bind _spline (`/Game/Cinematics/ObjectsForCinematics/BP_Spline.Spline` (`self.SplinePath`)))
  (bind _returnvalue (* `Set Move Alpha` (`SplineComponent.GetSplineLength` _spline)))
  (`self.K2_SetActorLocationAndRotation` (`SplineComponent.GetLocationAtDistanceAlongSpline` _spline _returnvalue "World") (`SplineComponent.GetRotationAtDistanceAlongSpline` _spline _returnvalue "World")))

(fn `OnRep_PositionState`
  (bind _positionstate (`self.PositionState`))
  (`KismetSystemLibrary.PrintString` (`KismetStringLibrary.Conv_DoubleToString` _positionstate))
  (`self.SetPositionState` _positionstate))

(fn `SetPositionState`
  (params (SetPosState :type "Float (double-precision)"))
  (`self.MoveEffigy` SetPosState))

(fn `UserConstructionScript`)