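; BP_CutsceneTrigger is a one-shot trigger volume that plays the LS_IntroToTheTown cinematic when the player enters it.
; On box overlap by an actor tagged Player, a DoOnce lets it disable the third-person character's input and play a newly created level sequence player.
; A delay equal to the sequence's duration then restores input, rather than a finished-event binding.
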(event `self.Box.OnComponentBeginOverlap`
  (params (OverlappedComponent :type "PrimitiveComponent Object Reference") (OtherActor :type "Actor Object Reference") (OtherComp :type "PrimitiveComponent Object Reference") (OtherBodyIndex :type Integer) (bFromSweep :type Boolean) (SweepResult :type "HitResult Structure (by ref)"))
  ; When you enter the zone, disable input and play a cinematic, once done return the controls to the player
  (if (`self.ActorHasTag` OtherActor "Player")
    (`/Engine/EditorBlueprintResources/StandardMacros.DoOnce` false
      (:`Completed`
        (bind _asbp_third_person_character (cast `/Game/ThirdPerson/Blueprints/BP_ThirdPersonCharacter` OtherActor))
        (`self.DisableInput` _asbp_third_person_character null)
        (bind (_outactor _returnvalue) (`LevelSequencePlayer.CreateLevelSequencePlayer` "/Game/Cinematics/Cutscenes(LevelSequences)/LS_IntroToTheTown.LS_IntroToTheTown"))
        (`MovieSceneSequencePlayer.Play` _returnvalue)
        (`KismetSystemLibrary.Delay` (`TimeManagementBlueprintLibrary.Conv_QualifiedFrameTimeToSeconds` (`MovieSceneSequencePlayer.GetDuration` _returnvalue)))
        (`self.EnableInput` _asbp_third_person_character null)))))

(fn `UserConstructionScript`)