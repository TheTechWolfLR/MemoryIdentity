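; BP_InteractableObject is a one-time interactable key item for the mission system.
; On first Interact it reports its ItemName to BP_GameInstance and marks itself as interacted.
; If an NPCGirl reference is valid, it repoints that NPC's BP_DialogueComponent to the Dialogue_Datatabel_Ahmet table and resets the starting row, changing the girl's dialogue.
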(event EventInteract
  (params (PlayerReffrence :type BP%20Third%20Person%20Character%20Object%20Reference))
  (bind _npc_girl (Variables|Default|GetNPC%20girl))
  (bind _returnvalue (Actor|GetComponentbyClass _npc_girl "/Game/DialogueShenanagins/BP_DialogueComponent.BP_DialogueComponent_C"))
  (if (not (Variables|Default|GetInteracted))
    (bind _asbp_game_instance (Utilities|Casting|CastToBP_GameInstance (Game|GetGameInstance)))
    (Default|InteractedwithKeyItem _asbp_game_instance (Variables|Default|GetItem%20Name))
    (Variables|Default|SetInteracted true)
    (Development|PrintString "Interact")
    ;[0.15 0.15 0.15 0.5] When you interact with this item, get the dialog component from the little girl and make it so it changes the dialog tabel from one to another
    (Utilities|IsValid _npc_girl
      (:Is%20Valid
        (Variables|/Game/DialogueShenanagins/BP_DialogueComponent.BP_DialogueComponent_C|SetData%20Table _returnvalue "/Game/DialogueShenanagins/ActualDialogue/Dialogue_Datatabel_Ahmet.Dialogue_Datatabel_Ahmet")
        (Variables|/Game/DialogueShenanagins/BP_DialogueComponent.BP_DialogueComponent_C|SetRow%20Name _returnvalue "1")
        (Development|PrintString "CHanged Girl's dialogue")))))