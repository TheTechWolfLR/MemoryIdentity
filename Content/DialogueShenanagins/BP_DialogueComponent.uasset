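; Dialogue component that runs branching, data-table-driven conversations for a named speaker.
; Interact opens WB_Dialogue or advances it, with each row supplying the text, next table and row, end flag and optional choices.
; Choices become WB_Options widgets holding a component reference, and OptionSelected jumps to a given row.
; Opening enables the mouse, ending or leaving restores game-only input, and the first interaction reports to BP_GameInstance via TalkedToPOI.
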(event `/Game/DialogueShenanagins/BP_Interact.LeaveDialogue`
  (bind _returnvalue (`GameplayStatics.GetPlayerController` 0))
  ; also end if you leave the area
  (`/Engine/EditorBlueprintResources/StandardMacros.IsValid` (`self.DialogueWidget`)
    (:`Is Valid`
      ; End Dialog when true
      (`Widget.RemoveFromParent` (`self.DialogueWidget`) :!label _label)
      (set `self.EndDialogue` false)
      (set `self.DialogueWidget` null)
      ; get rid of the mouse and enter play
      (`WidgetBlueprintLibrary.SetInputMode_GameOnly` _returnvalue)
      (set `PlayerController.bShowMouseCursor` false _returnvalue))))

(event `Option Selected`
  (params (Table :type "DataTable Object Reference") (RowName :type Name))
  (bind _dialoguewidget (`self.DialogueWidget`))
  ; When an option is selected, keep it going
  (bind _returnvalue (`|GetDataTableRow` Table RowName)
    (:`then`
      (`PanelWidget.ClearChildren` (`/Game/DialogueShenanagins/WB_Dialogue.OptionScrollBox` _dialoguewidget))
      (bind (_dialogue _row _datatable _enddialogue _options_ _openendedoptions) (break `/Game/DialogueShenanagins/Dialogue_Structure` _returnvalue))
      (`/Game/DialogueShenanagins/WB_Dialogue.Update Dialogue` _dialoguewidget _dialogue)
      (set `self.Row Name` _row)
      (set `self.Data Table` _datatable)
      (set `self.EndDialogue` _enddialogue)
      ; If it has options, display them
      (if _options_
        (for _array_element _openendedoptions
          (bind (_optionname _row_2 _datatable_2) (break `/Game/DialogueShenanagins/DialogOptions_Structure` _array_element))
          (bind _returnvalue_2 (`|CreateWidget` "/Game/DialogueShenanagins/WB_Options.WB_Options_C" null (`KismetTextLibrary.Conv_NameToText` _optionname) self _row_2 _datatable_2))
          (`PanelWidget.AddChild` (`/Game/DialogueShenanagins/WB_Dialogue.OptionScrollBox` (`self.DialogueWidget`)) _returnvalue_2))))
    (:`RowNotFound`
      (`KismetSystemLibrary.PrintString` "Selected option row not found"))))

(event `self.ReceiveBeginPlay`
  (add `self.OnFirstInteraction` (delegate `OnFirstInteraction_Event`)))

(event `/Game/DialogueShenanagins/BP_Interact.Interact`
  (params (PlayerReffrence :type "/Game/ThirdPerson/Blueprints/BP_ThirdPersonCharacter Object Reference"))
  (bind _returnvalue (`GameplayStatics.GetPlayerController` 0))
  (if (not (`self.HasInteracted`))
    (`self.OnFirstInteraction`)
    (set `self.HasInteracted` true))
  (if (`self.EndDialogue`)
    (goto _label)
    (else
      (`/Engine/EditorBlueprintResources/StandardMacros.IsValid` (`self.DialogueWidget`)
        (:`Is Valid`
          ; Keep it going if it keeps going
          (bind _returnvalue_2 (`|GetDataTableRow` (`self.Data Table`) (`self.Row Name`))
            (:`then`
              (bind (_dialogue _row _datatable _enddialogue _options_ _openendedoptions) (break `/Game/DialogueShenanagins/Dialogue_Structure` _returnvalue_2))
              (`/Game/DialogueShenanagins/WB_Dialogue.Update Dialogue` (`self.DialogueWidget`) _dialogue)
              (set `self.Row Name` _row)
              (set `self.Data Table` _datatable)
              (set `self.EndDialogue` _enddialogue)
              (set `self.Open Ended Options` _openendedoptions))))
        (:`Is Not Valid`
          ; Create a dialog widget for the dialog
          (bind _returnvalue_3 (`|GetDataTableRow` (`self.Data Table`) (`self.Row Name`))
            (:`then`
              (bind (_dialogue_2 _row_2 _datatable_2 _enddialogue_2 _options__2 _openendedoptions_2) (break `/Game/DialogueShenanagins/Dialogue_Structure` _returnvalue_3))
              (bind _returnvalue_4 (`|CreateWidget` "/Game/DialogueShenanagins/WB_Dialogue.WB_Dialogue_C" null (`KismetTextLibrary.Conv_NameToText` (`self.Name`)) _dialogue_2))
              (bind _output_get (set `self.DialogueWidget` _returnvalue_4))
              (`UserWidget.AddToViewport` _output_get 0)
              (set `self.Row Name` _row_2)
              (set `self.Data Table` _datatable_2)
              (set `self.EndDialogue` _enddialogue_2)
              (set `self.Open Ended Options` _openendedoptions_2)
              ; Show mouse so you can select (maybe change to controler support if possible)
              (`WidgetBlueprintLibrary.SetInputMode_GameAndUIEx` _returnvalue null)
              (set `PlayerController.bShowMouseCursor` true _returnvalue)))))
      ; If it has options, display them
      (if (or _options_ _options__2)
        (for _array_element (`self.Open Ended Options`)
          (bind (_optionname _row_3 _datatable_3) (break `/Game/DialogueShenanagins/DialogOptions_Structure` _array_element))
          (bind _returnvalue_5 (`|CreateWidget` "/Game/DialogueShenanagins/WB_Options.WB_Options_C" null (`KismetTextLibrary.Conv_NameToText` _optionname) self _row_3 _datatable_3))
          (`PanelWidget.AddChild` (`/Game/DialogueShenanagins/WB_Dialogue.OptionScrollBox` (`self.DialogueWidget`)) _returnvalue_5))))))

(event `OnFirstInteraction_Event`
  (`KismetSystemLibrary.PrintString` "Hello")
  (bind _asbp_game_instance (cast `/Game/Chrono_MissionBPs/BP_GameInstance` (`GameplayStatics.GetGameInstance`)))
  (`/Game/Chrono_MissionBPs/BP_GameInstance.TalkedToPOI` _asbp_game_instance (`self.Name`)))